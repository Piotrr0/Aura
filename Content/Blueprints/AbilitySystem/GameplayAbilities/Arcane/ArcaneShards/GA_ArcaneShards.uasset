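; Gameplay ability for Arcane Shards that shows a magic circle, waits for an input press and spawns shards around the point under the mouse.
; A spawned BP_PointCollection supplies ground points at a random yaw around the targeted location, and the magic circle is then hidden.
; A looping timer fires one GameplayCue per point, then destroys the collection and ends the ability after a short delay.
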(event `self.K2_ActivateAbility`
  (`|ExecutionSequence`
    (:`then_0`
      (message `PlayerInterface.ShowMagicCircle` (`self.GetAvatarActorFromActorInfo`) null))
    (:`then_1`
      (`AbilityTask_WaitInputPress.WaitInputPress` false
        (:`OnPress`
          (bind (_asynctaskproxy _data) (`TargetDataUnderMouse.CreateTargetDataUnderMouse`)
            (:`ValidData`
              (bind (_bblockinghit _binitialoverlap _time _distance _location _impactpoint) (`GameplayStatics.BreakHitResult` (`AbilitySystemBlueprintLibrary.GetHitResultFromTargetData` _data)))
              (bind _returnvalue (`|SpawnActorFromClass` "/Game/Blueprints/AbilitySystem/GameplayAbilities/Arcane/ArcaneShards/BP_PointCollection.BP_PointCollection_C" (`KismetMathLibrary.Conv_VectorToTransform` _impactpoint) "AlwaysSpawn" "MultiplyWithRoot" null null))
              (set `self.PointCollection` _returnvalue)
              (set `self.GroundPoints` (`PointCollection.GetGroundPoints` _returnvalue _impactpoint (`self.NumPoints`) (`KismetMathLibrary.RandomFloatInRange` 0.0 360.0)))
              (bind _returnvalue_2 (`KismetSystemLibrary.K2_SetTimerDelegate` (delegate `SpawnShard`) (`self.ShardSpawnDeltaTime`) true))
              (set `self.ShardSpawnTimer` _returnvalue_2)
              (`self.SpawnShard`)
              (message `PlayerInterface.HideMagicCircle` (`self.GetAvatarActorFromActorInfo`)))))))))

(event `SpawnShard`
  (if (< (`self.Count`) (`self.NumPoints`))
    (set `self.ShardSpawnLocation` (`SceneComponent.K2_GetComponentLocation` (`|GetArrayItem` (`self.GroundPoints`) (`self.Count`))))
    (`/Engine/EditorBlueprintResources/StandardMacros.IncrementInt` (`self.Count`)
      (:`  `
        (`self.K2_ExecuteGameplayCueWithParams` (struct :`TagName` "GameplayCue.ArcaneShards") (`AbilitySystemBlueprintLibrary.MakeGameplayCueParameters` 0.0 0.0 (struct) (struct) (struct) (struct) (struct) (`self.ShardSpawnLocation`)))))
    (else
      (`KismetSystemLibrary.K2_ClearAndInvalidateTimerHandle` (`self.ShardSpawnTimer`))
      (`KismetSystemLibrary.Delay` 0.2)
      (`Actor.K2_DestroyActor` (`self.PointCollection`))
      (`self.K2_EndAbility`))))