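; Base gameplay ability for passive spells that repeatedly applies a gameplay effect to its owner.
; On activation it starts a looping timer at the Period interval, and each tick applies the PassiveEffect class at level 1 and prints a debug string.
; Ending the ability clears and invalidates the timer.
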(event `self.K2_ActivateAbility`
  (bind _returnvalue (`KismetSystemLibrary.K2_SetTimerDelegate` (delegate `PassiveAbilityEvent`) (`self.Period`) true))
  (set `self.PeriodTimer` _returnvalue))

(event `PassiveAbilityEvent`
  (`self.K2_ApplyGameplayEffectSpecToOwner` (`self.MakeOutgoingGameplayEffectSpec` (`self.PassiveEffect`)))
  (`KismetSystemLibrary.PrintString` "Effect applied"))

(event `self.K2_OnEndAbility`
  (params (bWasCancelled :type Boolean))
  (`KismetSystemLibrary.K2_ClearAndInvalidateTimerHandle` (`self.PeriodTimer`)))