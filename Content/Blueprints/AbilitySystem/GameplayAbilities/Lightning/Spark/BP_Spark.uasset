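; BP_Spark is a lightning ability spark actor that wanders erratically across the horizontal plane.
; From BeginPlay it loops on a random short delay, each time resetting the ProjectileMovement velocity to a random XY heading scaled by InitialSpeed, with zero Z.
; RandomUnitVector2 normalizes a cosine and sine of separately rolled angles spanning 0 to 260 degrees, so headings are not uniformly distributed.
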(event `self.ReceiveBeginPlay`
  (bind (_returnvalue_x _returnvalue_y) (`KismetMathLibrary.BreakVector2D` (* (`self.RandomUnitVector2`) (`ProjectileMovementComponent.InitialSpeed` (`self.ProjectileMovement`)))))
  (`KismetSystemLibrary.Delay` (`KismetMathLibrary.RandomFloatInRange` 0.5 1.5) :!label _label)
  (set `MovementComponent.Velocity` (`KismetMathLibrary.MakeVector` _returnvalue_x _returnvalue_y) (`self.ProjectileMovement`))
  (goto _label))

(fn `RandomUnitVector2`
  (returns (Vector2 :type "Vector2D Structure"))
  (bind _returnvalue (`KismetMathLibrary.RandomFloatInRange` 0.0 260.0))
  (return (`KismetMathLibrary.Normal2D` (`KismetMathLibrary.MakeVector2D` (`KismetMathLibrary.DegCos` _returnvalue) (`KismetMathLibrary.DegSin` _returnvalue)))))

(fn `UserConstructionScript`)